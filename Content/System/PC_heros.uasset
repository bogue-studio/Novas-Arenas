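; PC_heros is the hero's player controller, which opens the main menu (inventory display) when the Menu input action is pressed.
; It disables character movement, then reuses or lazily creates the W_MainMenu widget, adds it to the viewport, shows the cursor and switches to UI-only input.
; StopMovement runs only when the widget already exists.
; CheckKey and the construction script are empty stubs.
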(event `InputAction|Menu` :paused true
  (params (Key :type "Key Structure"))
  (bind _returnvalue (`GameplayStatics.GetPlayerController` 0))
  (bind _returnvalue_2 (`GameplayStatics.GetPlayerController` 0))
  ;[1 1 1] Affichage de l'inventaireV2
  (:`Pressed`
    (`CharacterMovementComponent.DisableMovement` (`Character.CharacterMovement` (`GameplayStatics.GetPlayerCharacter` 0)))
    (`/Engine/EditorBlueprintResources/StandardMacros.IsValid` (`self.MainMenu`)
      (:`Is Valid`
        (`UserWidget.AddToViewport` (`self.MainMenu`) 0)
        (set `PlayerController.bShowMouseCursor` true _returnvalue)
        (`WidgetBlueprintLibrary.SetInputMode_UIOnlyEx` _returnvalue (`self.MainMenu`))
        (`self.StopMovement`))
      (:`Is Not Valid`
        (bind _returnvalue_3 (`|CreateWidget` "/Game/System/UserWidget/Menu/W_MainMenu.W_MainMenu_C"))
        (bind _output_get (set `self.MainMenu` _returnvalue_3))
        (`UserWidget.AddToViewport` _output_get 0)
        (set `PlayerController.bShowMouseCursor` true _returnvalue_2)
        (`WidgetBlueprintLibrary.SetInputMode_UIOnlyEx` _returnvalue_2 (`self.MainMenu`))))))

(fn `CheckKey`
  (params (Key :type "Key Structure" :default "None")))

(fn `UserConstructionScript`)