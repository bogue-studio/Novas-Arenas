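; PC_heros is the hero's player Blueprint that shows and hides the main menu, labeled as the V2 inventory display.
; The Menu input action drives a FlipFlop that alternates between opening and closing the menu.
; Opening creates W_MainMenu on first use, caches it for reuse, adds it to the viewport and shows the mouse cursor.
; Closing removes the widget from its parent and hides the cursor.
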(event `InputAction|Menu` :paused true
  (params (Key :type "Key Structure"))
  ;[1 1 1] Affichage de l'inventaireV2
  (:`Pressed`
    (`/Engine/EditorBlueprintResources/StandardMacros.FlipFlop`
      (:`A`
        (`/Engine/EditorBlueprintResources/StandardMacros.IsValid` (`self.MainMenu`)
          (:`Is Valid`
            (`UserWidget.AddToViewport` (`self.MainMenu`) 0)
            (set `PlayerController.bShowMouseCursor` true (`GameplayStatics.GetPlayerController` 0)))
          (:`Is Not Valid`
            (bind _returnvalue (`|CreateWidget` "/Game/Gameplay/UserWidget/Menu/W_MainMenu.W_MainMenu_C"))
            (bind _output_get (set `self.MainMenu` _returnvalue))
            (`UserWidget.AddToViewport` _output_get 0)
            (set `PlayerController.bShowMouseCursor` true (`GameplayStatics.GetPlayerController` 0)))))
      (:`B`
        (`Widget.RemoveFromParent` (`self.MainMenu`))
        (set `PlayerController.bShowMouseCursor` false (`GameplayStatics.GetPlayerController` 0))))))

(fn `UserConstructionScript`)