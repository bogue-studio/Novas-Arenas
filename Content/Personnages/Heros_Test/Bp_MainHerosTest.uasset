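; Test hero Character with movement, TPS/FPS camera switching, crouch, jump, sprint, health clamping and a pause menu.
; A looping timer drives GestionEndurance, draining stamina during jump or sprint and regenerating it otherwise.
; Tick line-traces from the FPS camera to set LookActor; E interacts with it and triggers dialogue on overlapping NPCs via BP_NpcInterface.
; Quest events create, complete and remove widgets in the QuestLog created at BeginPlay.
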(event `InputAxis|MoveForward`
  (params (AxisValue :type "Float (single-precision)"))
  ;[1 1 1] Déplacements
  (`self.AddMovementInput` (`KismetMathLibrary.GetForwardVector` (`KismetMathLibrary.MakeRotator` 0.0 0.0 (.yaw (`self.GetControlRotation`)))) AxisValue))

(event `self.ReceiveBeginPlay`
  (bind _returnvalue (`|CreateWidget` "/Game/System/QuestSystem/BP_QuestLog.BP_QuestLog_C"))
  (bind _output_get (set `self.QuestLog` _returnvalue))
  (`UserWidget.AddToViewport` _output_get 0))

(event `InputAxis|MoveRight`
  (params (AxisValue :type "Float (single-precision)"))
  ;[1 1 1] Déplacements
  (`self.AddMovementInput` (`KismetMathLibrary.GetRightVector` (`KismetMathLibrary.MakeRotator` 0.0 0.0 (.yaw (`self.GetControlRotation`)))) AxisValue))

(event `InputAction|SwitchCamera`
  (params (Key :type "Key Structure"))
  ;[1 1 1] Changement de vue TPS FPS
  (:`Pressed`
    (`self.ChangerCamera`)))

(event `InputAction|crouch`
  (params (Key :type "Key Structure"))
  ;[1 1 1] gestion du crouch
  (:`Pressed`
    (`self.Crouch`))
  (:`Released`
    (`self.UnCrouch`)))

(event `InputAction|Jump`
  (params (Key :type "Key Structure"))
  ;[1 1 1] gestion du saut
  (:`Pressed`
    (if (> (`self.Endurance`) 30.0)
      (`self.Jump`)
      (set `self.MyTimer` 0.2)
      (set `self.is_jumping` true)
      (`self.GestionEndurance` :!label _label)
      (`KismetSystemLibrary.K2_SetTimer` null "GestionEndurance" (`self.MyTimer`) true)))
  (:`Released`
    (`self.StopJumping`)
    (set `self.MyTimer` 0.2)
    (set `self.is_jumping` false)
    (goto _label)))

(event `InputAxis|Turn`
  (params (AxisValue :type "Float (single-precision)"))
  ;[1 1 1] Orientation de la caméra
  (`self.AddControllerYawInput` AxisValue))

(event `InputAction|sprint`
  (params (Key :type "Key Structure"))
  ;[1 1 1] Sprint
  (:`Pressed`
    (set `CharacterMovementComponent.MaxWalkSpeed` 1000.0 (`self.CharacterMovement`))
    (set `self.MyTimer` 0.2)
    (bind _returnvalue (`KismetSystemLibrary.K2_SetTimer` null "GestionEndurance" (`self.MyTimer`) true :!label _label_2))
    (set `self.timerEndurance` _returnvalue))
  (:`Released`
    (set `CharacterMovementComponent.MaxWalkSpeed` 280.75 (`self.CharacterMovement`))
    (set `self.MyTimer` 0.2)
    (goto _label_2)))

(event `Key|P` :paused true
  (params (Key :type "Key Structure"))
  ;[1 1 1] Pause Menu
  (:`Pressed`
    (`/Engine/EditorBlueprintResources/StandardMacros.FlipFlop`
      (:`A`
        (`WidgetBlueprintLibrary.SetInputMode_UIOnlyEx` (`GameplayStatics.GetPlayerController` 0) (`self.W_PauseRef`))
        (`GameplayStatics.SetGamePaused` true)
        (bind _returnvalue (`|CreateWidget` "/Game/System/Pause/W_Pause.W_Pause_C"))
        (bind _output_get (set `self.W_PauseRef` _returnvalue))
        (`UserWidget.AddToViewport` _output_get 0)
        (set `PlayerController.bShowMouseCursor` true (`GameplayStatics.GetPlayerController` 0)))
      (:`B`
        (`WidgetBlueprintLibrary.SetInputMode_GameOnly` (`GameplayStatics.GetPlayerController` 0))
        (`GameplayStatics.SetGamePaused` false)
        (`Widget.RemoveFromParent` (`self.W_PauseRef`))))))

(event `InputAxis|LookUp`
  (params (AxisValue :type "Float (single-precision)"))
  ;[1 1 1] Orientation de la caméra
  (`self.AddControllerPitchInput` AxisValue))

(event `self.ReceiveTick`
  (params (DeltaSeconds :type "Float (single-precision)"))
  (`self.IntercationV2`))

(event `Key|E`
  (params (Key :type "Key Structure"))
  ;[1 1 1] Test si l'objet est détecté ou non et ajout
  (:`Pressed`
    (bind _lookactor (`self.LookActor`)
      (:`then`
        (bind _success (message `/Game/System/InventorySystemV2/InteractionInterface.InteractWith` _lookactor self))
        (if _success
          (bind _keys (`BlueprintMapLibrary.Map_Keys` (`/Game/System/InventorySystemV2/InventoryComponent.InventoryContent` (`self.InventoryComponent`))))
          (`KismetSystemLibrary.PrintString` (`KismetStringLibrary.Conv_NameToString` (`|GetArrayItem` _keys)))))
      (:`else`))))

(event `AcceptQuest`
  (params (QuestInfo :type "/Game/System/QuestSystem/QuestInfo Structure"))
  (bind (_questname _questdescription) (break `/Game/System/QuestSystem/QuestInfo` QuestInfo))
  ;[1 1 1] AcceptQuest
  (bind _returnvalue (`|CreateWidget` "/Game/System/QuestSystem/BP_Quest.BP_Quest_C"))
  (set `/Game/System/QuestSystem/BP_Quest.QuestInfo` QuestInfo _returnvalue)
  (`KismetArrayLibrary.Array_Add` (`self.ActiveQuests`) _returnvalue)
  (`TextBlock.SetText` (`/Game/System/QuestSystem/BP_Quest.QuestName` _returnvalue) _questname)
  (`TextBlock.SetText` (`/Game/System/QuestSystem/BP_Quest.Description` _returnvalue) _questdescription)
  (`VerticalBox.AddChildToVerticalBox` (`/Game/System/QuestSystem/BP_QuestLog.QuestHolder` (`self.QuestLog`)) _returnvalue))

(event `QuestComplete`
  (params (ActiveQuest :type "/Game/System/QuestSystem/BP_Quest Object Reference"))
  ;[1 1 1] Quest Complete - Update Values
  (`TextBlock.SetText` (`/Game/System/QuestSystem/BP_Quest.Complete?` ActiveQuest) "- Complete!"))

(event `Key|E`
  (params (Key :type "Key Structure"))
  ;[1 1 1] Interaction Quest and dialog
  (:`Pressed`
    (for _array_element (`self.GetOverlappingActors` "/Script/Engine.Actor")
      (if (`KismetSystemLibrary.DoesImplementInterface` _array_element "/Game/Personnages/NPC/BP_NpcInterface.BP_NpcInterface_C")
        (message `/Game/Personnages/NPC/BP_NpcInterface.ActiveDialog` _array_element (`self.ActiveQuests`))
        (break)))))

(event `RemoveQuest`
  (params (ActiveQuest :type "/Game/System/QuestSystem/BP_Quest Object Reference"))
  ;[1 1 1] Remove Quest From Variables
  (`Widget.RemoveFromParent` ActiveQuest)
  (`KismetArrayLibrary.Array_RemoveItem` (`self.ActiveQuests`) ActiveQuest))

(fn `ChangerCamera`
  (`ActorComponent.ToggleActive` (`self.CameraTPS`))
  (`ActorComponent.ToggleActive` (`self.CameraFPS`))
  (if (`ActorComponent.IsActive` (`self.CameraFPS`))
    (set `Pawn.bUseControllerRotationYaw` true (`GameplayStatics.GetPlayerPawn` 0))
    (else
      (set `Pawn.bUseControllerRotationYaw` false (`GameplayStatics.GetPlayerPawn` 0))))
  (`SceneComponent.ToggleVisibility` (`self.Mesh`) false))

(fn `GestionEndurance`
  (if (`self.is_jumping`)
    ;[0.6795 1 0.7305] supression points endu
    (if (> (`self.Endurance`) 2.0)
      (set `self.Endurance` (- (`self.Endurance`) 2.0)))
    (elif (`MovementComponent.IsExceedingMaxSpeed` (`self.CharacterMovement`) 280.75)
      ;[0.6795 1 0.7305] supression points endu
      (if (> (`self.Endurance`) 0.0)
        (set `self.Endurance` (- (`self.Endurance`) 0.5))
        (else
          ;[1 1 1] arret du srpint
          (set `CharacterMovementComponent.MaxWalkSpeed` 280.75 (`self.CharacterMovement`))))
      (elif (< (`self.Endurance`) (`self.Endurance_Max`))
        ;[0.6795 1 0.7305] regen endurance
        (set `self.Endurance` (+ (`self.Endurance`) 1.0))
        (else
          ;[1 1 1] Pause du Timer
          (`KismetSystemLibrary.K2_PauseTimerHandle` (`self.timerEndurance`)))))))

(fn `GestionVie`
  (params (Points :type "Float (double-precision)"))
  (bind _output_get (set `self.Vie` (`KismetMathLibrary.FClamp` (+ (`self.Vie`) Points) 0.0 (`self.Vie_Max`))))
  (if (== _output_get 0.0)
    _))

(fn `IntercationV2`
  (bind _camerafps (`self.CameraFPS`))
  (bind _camerafps_2 (`self.CameraFPS`))
  (bind (_outhit _returnvalue) (`KismetSystemLibrary.LineTraceSingle` (+ (`SceneComponent.K2_GetComponentLocation` _camerafps_2) (* (`SceneComponent.GetForwardVector` _camerafps_2) 10)) (+ (`SceneComponent.K2_GetComponentLocation` _camerafps) (* (`SceneComponent.GetForwardVector` _camerafps) 400)) "TraceTypeQuery3"))
  (if _returnvalue
    (bind (_bblockinghit _binitialoverlap _time _distance _location _impactpoint _normal _impactnormal _physmat _hitactor) (`GameplayStatics.BreakHitResult` _outhit))
    (if (!= (`self.LookActor`) _hitactor)
      (bind _output_get (set `self.LookActor` _hitactor))
      (bind _message (message `/Game/System/InventorySystemV2/InteractionInterface.LookAt` _output_get self))
      (`KismetSystemLibrary.PrintString` (`KismetTextLibrary.Conv_TextToString` _message)))
    (else
      (set `self.LookActor` null))))

(fn `MouseInput`
  (bind _returnvalue (`GameplayStatics.GetPlayerController` 0))
  (if (`self.MouseVisibility`)
    (set `PlayerController.bShowMouseCursor` false _returnvalue)
    (`WidgetBlueprintLibrary.SetInputMode_GameOnly` _returnvalue)
    (set `self.MouseVisibility` false)
    (else
      (set `PlayerController.bShowMouseCursor` true _returnvalue)
      (`WidgetBlueprintLibrary.SetInputMode_GameAndUIEx` _returnvalue null)
      (set `self.MouseVisibility` true))))

(fn `OnEndDialogue`
  (returns (Success :type Boolean))
  (return false))

(fn `OnReturnDialogueOption`
  (params (ReturnOption :type String))
  (returns (Success :type Boolean))
  (return false))

(fn `TalkTo`
  (params (Instigator :type "Actor Object Reference") (Dialogue :type Name))
  (returns (Success :type Boolean))
  (return false))

(fn `UserConstructionScript`)