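; BP_Arme is a weapon the hero can pick up and fire.
; Overlapping its box enables player input on it, so E can attach it to a kalash socket, or to the back socket when IsWearing is already true.
; The E action also passes its class to the hero's Arme child actor component.
; Tirer spawns an actor at the Sphere's transform, passing initial and maximum speed.
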(event `self.Box.OnComponentBeginOverlap`
  (params (OverlappedComponent :type "PrimitiveComponent Object Reference") (OtherActor :type "Actor Object Reference") (OtherComp :type "PrimitiveComponent Object Reference") (OtherBodyIndex :type Integer) (bFromSweep :type Boolean) (SweepResult :type "HitResult Structure (by ref)"))
  (bind _asue_4asp_character (cast `` OtherActor))
  (set `self.Heros_Ref` null _asue_4asp_character)
  (`self.EnableInput` (`GameplayStatics.GetPlayerController` 0)))

(event `Key|E`
  (params (Key :type "Key Structure"))
  (:`Pressed`
    (if (`self.isWearing`)
      (`self.K2_AttachToComponent` null "SK_kalash-dos" "SnapToTarget" "SnapToTarget" "SnapToTarget")
      (else
        (`self.K2_AttachToComponent` null "SK_kalash" "SnapToTarget" "SnapToTarget" "SnapToTarget")
        (set `self.isWearing` true)))
    (`ChildActorComponent.SetChildActorClass` (`/Game/Weapon/BP_Arme.arme` (`.Heros_Ref` (`self.Heros_Ref`))) (`GameplayStatics.GetObjectClass` self))))

(fn `tirer`
  (`|SpawnActorFromClass` null (`SceneComponent.K2_GetComponentToWorld` (`self.Sphere`)) "Undefined" "OverrideRootScale" null (`self.Initial_Speed`) (`self.Max_Speed`) null))

(fn `UserConstructionScript`)