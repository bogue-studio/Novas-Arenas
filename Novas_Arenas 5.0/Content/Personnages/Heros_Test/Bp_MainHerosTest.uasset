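; Test main hero character with camera-relative movement, look, crouch, jump, sprint and a TPS/FPS camera toggle that also switches controller yaw and mesh visibility.
; BeginPlay calls GI_Heros to set up the main UI.
; Jump and sprint start a looping GestionEndurance timer that drains stamina, ends sprint when empty, or regenerates until full and pauses.
; GestionVie clamps health changes, with no handling at zero yet.
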(event `InputAxis|MoveForward`
  (params (AxisValue :type "Float (single-precision)"))
  ;[1 1 1] Déplacements
  (`self.AddMovementInput` (`KismetMathLibrary.GetForwardVector` (`KismetMathLibrary.MakeRotator` 0.0 0.0 (.yaw (`self.GetControlRotation`)))) AxisValue))

(event `self.ReceiveBeginPlay`
  ;[1 1 1] Afficher UI
  (bind _asgi_heros (cast `/Game/System/Gi_heros` (`GameplayStatics.GetGameInstance`)))
  (`/Game/System/Gi_heros.Gestion_UIMain` _asgi_heros))

(event `InputAxis|MoveRight`
  (params (AxisValue :type "Float (single-precision)"))
  ;[1 1 1] Déplacements
  (`self.AddMovementInput` (`KismetMathLibrary.GetRightVector` (`KismetMathLibrary.MakeRotator` 0.0 0.0 (.yaw (`self.GetControlRotation`)))) AxisValue))

(event `InputAction|SwitchCamera`
  (params (Key :type "Key Structure"))
  ;[1 1 1] Changement de vue TPS FPS
  (:`Pressed`
    (`self.ChangerCamera`)))

(event `InputAction|crouch`
  (params (Key :type "Key Structure"))
  ;[1 1 1] gestion du crouch
  (:`Pressed`
    (`self.Crouch`))
  (:`Released`
    (`self.UnCrouch`)))

(event `InputAction|Jump`
  (params (Key :type "Key Structure"))
  ;[1 1 1] gestion du saut
  (:`Pressed`
    (if (> (`self.Endurance`) 30.0)
      (`self.Jump`)
      (set `self.MyTimer` 0.2)
      (set `self.is_jumping` true)
      (`self.GestionEndurance` :!label _label)
      (`KismetSystemLibrary.K2_SetTimer` null "GestionEndurance" (`self.MyTimer`) true)))
  (:`Released`
    (`self.StopJumping`)
    (set `self.MyTimer` 0.2)
    (set `self.is_jumping` false)
    (goto _label)))

(event `InputAxis|Turn`
  (params (AxisValue :type "Float (single-precision)"))
  ;[1 1 1] Orientation de la caméra
  (`self.AddControllerYawInput` AxisValue))

(event `InputAction|sprint`
  (params (Key :type "Key Structure"))
  ;[1 1 1] Sprint
  (:`Pressed`
    (set `CharacterMovementComponent.MaxWalkSpeed` 375.0 (`self.CharacterMovement`))
    (set `self.MyTimer` 0.2)
    (bind _returnvalue (`KismetSystemLibrary.K2_SetTimer` null "GestionEndurance" (`self.MyTimer`) true :!label _label_2))
    (set `self.timerEndurance` _returnvalue))
  (:`Released`
    (set `CharacterMovementComponent.MaxWalkSpeed` 93.75 (`self.CharacterMovement`))
    (set `self.MyTimer` 0.2)
    (goto _label_2)))

(event `InputAxis|LookUp`
  (params (AxisValue :type "Float (single-precision)"))
  ;[1 1 1] Orientation de la caméra
  (`self.AddControllerPitchInput` AxisValue))

(fn `ChangerCamera`
  (`ActorComponent.ToggleActive` (`self.CameraTPS`))
  (`ActorComponent.ToggleActive` (`self.CameraFPS`))
  (if (`ActorComponent.IsActive` (`self.CameraFPS`))
    (set `Pawn.bUseControllerRotationYaw` true (`GameplayStatics.GetPlayerPawn` 0))
    (else
      (set `Pawn.bUseControllerRotationYaw` false (`GameplayStatics.GetPlayerPawn` 0))))
  (`SceneComponent.ToggleVisibility` (`self.Mesh`) false))

(fn `GestionEndurance`
  (if (`self.is_jumping`)
    ;[0.6795 1 0.7305] supression points endu
    (if (> (`self.Endurance`) 30.0)
      (set `self.Endurance` (- (`self.Endurance`) 30.0)))
    (elif (`MovementComponent.IsExceedingMaxSpeed` (`self.CharacterMovement`) 93.75)
      ;[0.6795 1 0.7305] supression points endu
      (if (> (`self.Endurance`) 0.0)
        (set `self.Endurance` (- (`self.Endurance`) 2.0))
        (else
          ;[1 1 1] arret du srpint
          (set `CharacterMovementComponent.MaxWalkSpeed` 93.75 (`self.CharacterMovement`))))
      (elif (< (`self.Endurance`) (`self.Endurance_Max`))
        ;[0.6795 1 0.7305] regen endurance
        (set `self.Endurance` (+ (`self.Endurance`) 1.0))
        (else
          ;[1 1 1] Pause du Timer
          (`KismetSystemLibrary.K2_PauseTimerHandle` (`self.timerEndurance`)))))))

(fn `GestionVie`
  (params (Points :type "Float (double-precision)"))
  (bind _output_get (set `self.Vie` (`KismetMathLibrary.FClamp` (+ (`self.Vie`) Points) 0.0 (`self.Vie_Max`))))
  (if (== _output_get 0.0)
    _))

(fn `UserConstructionScript`)